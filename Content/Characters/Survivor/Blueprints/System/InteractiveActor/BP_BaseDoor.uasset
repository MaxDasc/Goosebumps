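; BP_BaseDoor is a base door actor that the survivor player opens with a left mouse click while standing inside its overlap area, if they hold the matching key.
; Begin and end overlap track the ThirdPersonCharacter, and the click checks its HasKey against the door's KeyChannel.
; On success a Rotate timeline swings the Door's relative yaw from a RotationZ offset; both outcomes print debug text.
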(event Custom|InteractDoor
  (params (TestObject :type Can%20Pickup%20Object%20Reference))
  ;[1 1 1] Door Animation
  (Variables|Private|SetOpen? true)
  (Utilities|Casting|CastToThirdPersonCharacter (Game|GetPlayerCharacter 0))
  (bind _rotateblend (Timeline|Rotate Play)
    (:Update
      (Transformation|SetRelativeRotation (Variables|Default|GetDoor) (Math|Rotator|MakeRotator 0.0 0.0 (+ _rotateblend (Variables|Default|GetRotation%20Z))) false false))))

(event EventBeginPlay
  ;[1 1 1] Begin Play
  (Input|EnableInput (Game|GetPlayerController 0)))

(event Collision|EventActorBeginOverlap
  (params (OtherActor :type Actor%20Object%20Reference))
  ;[1 1 1] Begin/End Overlap
  (bind _asthird_person_character (Utilities|Casting|CastToThirdPersonCharacter OtherActor))
  (Variables|Default|SetIsInsideDoor true))

(event EventTick
  (params (DeltaSeconds :type Float%20%28single-precision%29)))

(event EventInteractionAction
  (params (Player :type Third%20Person%20Character%20Object%20Reference))
  ;[1 1 1] If interaction player to open door
  (Utilities|IsValid Player
    (:Is%20Valid
      (if (Default|HasKey Player (Variables|Constants|GetKeyChannel))
        (Development|PrintString "Open")
        (CallFunction|InteractDoor)
        (else
          (Development|PrintString "Dont Open"))))))

(event Collision|EventActorEndOverlap
  (params (OtherActor :type Actor%20Object%20Reference))
  ;[1 1 1] Begin/End Overlap
  (Utilities|Casting|CastToThirdPersonCharacter OtherActor)
  (Variables|Default|SetIsInsideDoor false))

(event Input|MouseEvents|LeftMouseButton
  (params (Key :type Key%20Structure :default "None"))
  ;[1 1 1] Open Door
  (:Pressed
    (if (Variables|Default|GetIsInsideDoor)
      (Default|InteractionAction self (stale Collision|EventActorBeginOverlap _asthird_person_character)))))

(fn ConstructionScript)